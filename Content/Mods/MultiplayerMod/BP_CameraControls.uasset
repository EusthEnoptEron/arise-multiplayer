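; BP_CameraControls is an actor in the multiplayer mod meant to dolly itself to keep a list of actors on screen.
; Its unconnected logic steps Distance in or out using AllVisible, then places the actor facing TargetLocation, but the offset direction is zero.
; AllVisible projects each actor through player 0's viewport via IsOnScreen, which applies width-based padding to both axes.
; Tick is empty, so none of this runs.
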(event EventBeginPlay)

(event Collision|EventActorBeginOverlap
  (params (OtherActor :type Actor%20Object%20Reference)))

(event EventTick
  (params (DeltaSeconds :type Float%20%28single-precision%29)))

(fn ConstructionScript)

(fn NewFunction0)

(fn AllVisible
  (params (Padding :type Float%20%28single-precision%29))
  (for _array_element (Variables|Default|GetActors)
    (bind _isonscreen (CallFunction|IsonScreen (Transformation|GetActorLocation _array_element) Padding))
    (if (not _isonscreen)
      (return false)))
  (return true))

(fn IsonScreen
  (params (Position :type Vector) (Padding :type Float%20%28single-precision%29))
  (bind _returnvalue (Viewport|GetViewportSize))
  (bind _returnvalue_2 (Viewport|GetViewportSize))
  (bind _returnvalue_3 (Game|GetPlayerController 0))
  (bind (_screenposition _returnvalue_4) (Class|GameplayStatics|ProjectWorldtoScreen _returnvalue_3 Position false))
  (bind (_x _y) (Math|Vector2D|BreakVector2D _returnvalue))
  (bind (_x_2 _y_2) (Math|Vector2D|BreakVector2D _returnvalue_2))
  (bind (_x_3 _y_3) (Math|Vector2D|BreakVector2D _screenposition))
  (LocalVariables|SetPaddingX (* Padding _x_2))
  (LocalVariables|SetPaddingY (* Padding _y_2))
  (if _returnvalue_4
    (return (Math|Boolean|ANDBoolean (>= _x_3 (LocalVariables|GetPaddingX)) (>= _y_3 (LocalVariables|GetPaddingX)) (<= (+ _x_3 (LocalVariables|GetPaddingX)) _x) (<= (+ _y_3 (LocalVariables|GetPaddingX)) _y)))
    (else
      (return false))))