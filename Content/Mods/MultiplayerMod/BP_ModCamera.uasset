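; BP_ModCamera is a multiplayer mod camera that keeps a group of actors on screen.
; While active, it eases its aim point toward the averaged targets and orbits it by input with clamped pitch.
; Two screen-padding thresholds drive zooming in and out, leaving a dead band between them.
; It feeds angle and focus overrides to MainCamera and sets the near clipping plane from the closest actor, releasing overrides on deactivation.
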(event Custom|OnCameraAngle
  (params (Value :type Vector%202D%20Structure))
  (bind _returnvalue (Utilities|Time|GetWorldDeltaSeconds))
  (bind _output_get (Variables|Default|SetCurrentInput Value))
  (Variables|Default|SetYawPitch (Math|Vector2D|MakeVector2D (Math|Rotator|NormalizeAxis (.X (Math|Vector2D|BreakVector2D (+ (* (Variables|Default|GetSpeed) (Math|Vector2D|MakeVector2D _returnvalue _returnvalue) _output_get) (Variables|Default|GetYawPitch))))) (Math|Float|Clamp(Float) (.Y (Math|Vector2D|BreakVector2D (+ (* (Variables|Default|GetSpeed) (Math|Vector2D|MakeVector2D _returnvalue _returnvalue) _output_get) (Variables|Default|GetYawPitch)))) -75.0 -1e+01)))
  (Variables|Default|SetCameraRotation (Math|Rotator|MakeRotator 0.0 (Math|Float|Clamp(Float) (.Y (Math|Vector2D|BreakVector2D (+ (* (Variables|Default|GetSpeed) (Math|Vector2D|MakeVector2D _returnvalue _returnvalue) _output_get) (Variables|Default|GetYawPitch)))) -75.0 -1e+01) (Math|Rotator|NormalizeAxis (.X (Math|Vector2D|BreakVector2D (+ (* (Variables|Default|GetSpeed) (Math|Vector2D|MakeVector2D _returnvalue _returnvalue) _output_get) (Variables|Default|GetYawPitch)))))))
  (Variables|Default|SetDirection (Math|Vector|GetForwardVector (Math|Rotator|MakeRotator 0.0 (Math|Float|Clamp(Float) (.Y (Math|Vector2D|BreakVector2D (+ (* (Variables|Default|GetSpeed) (Math|Vector2D|MakeVector2D _returnvalue _returnvalue) _output_get) (Variables|Default|GetYawPitch)))) -75.0 -1e+01) (Math|Rotator|NormalizeAxis (.X (Math|Vector2D|BreakVector2D (+ (* (Variables|Default|GetSpeed) (Math|Vector2D|MakeVector2D _returnvalue _returnvalue) _output_get) (Variables|Default|GetYawPitch)))))))))

(event EventBeginPlay)

(event Collision|EventActorBeginOverlap
  (params (OtherActor :type Actor%20Object%20Reference)))

(event EventTick
  (params (DeltaSeconds :type Float%20%28single-precision%29))
  (Variables|Default|SetTickDelta DeltaSeconds)
  (if (and (Math|Conversions|ToBoolean(Integer) (Utilities|Array|Length (Variables|Default|GetActors))) (Math|Conversions|ToBoolean(Integer) (Utilities|Array|Length (Variables|Default|GetTargets))))
    (Utilities|IsValid (Variables|Default|GetMainCamera)
      (:Is%20Valid
        (bind _aimpoint (CallFunction|GetAimPoint))
        (if (Math|Vector|Equal(Vector) (Variables|Default|GetCurrentAimPoint) "0, 0, 0" 0.0001) ; Set aim point directly when uninitialized
          (Variables|Default|SetCurrentAimPoint _aimpoint)
          (else
            (Variables|Default|SetCurrentAimPoint (Math|Vector|Lerp(Vector) (Variables|Default|GetCurrentAimPoint) _aimpoint (* (Variables|Default|GetTickDelta) 1e+01)))))
        (CallFunction|UpdateLocation true)
        (bind _visible (CallFunction|AllVisible 0.2))
        (if _visible ; Are all actors visible with a hefty padding?
          (Variables|Default|SetDistance (Math|Float|Max(Float) (- (Variables|Default|GetDistance) (* (Variables|Default|GetTickDelta) (Variables|Default|GetStepSpeed))) (Variables|Default|GetMinDistance)))
          (CallFunction|UpdateLocation true :!label _label)
          (else
            (bind _visible_2 (CallFunction|AllVisible 0.1)) ; Perhaps they're visible with less padding?
            (if _visible_2
              _
              (else
                (Variables|Default|SetDistance (+ (Variables|Default|GetDistance) (* (Variables|Default|GetTickDelta) (Variables|Default|GetStepSpeed))))
                (goto _label)))))
        (bind _distance (CallFunction|CalculateClippingDistance))
        (Default|NativeSetNearClippingPlane (Variables|Default|GetMod) _distance)))))

(fn ConstructionScript
  (Actor|Tick|SetActorTickEnabled false))

(fn AllVisible
  (params (Padding :type Float%20%28single-precision%29))
  (for _array_element (Variables|Default|GetActors)
    (bind _isonscreen (CallFunction|IsonScreen (Transformation|GetActorLocation _array_element) Padding))
    (if (not _isonscreen)
      (return false)))
  (return true))

(fn IsonScreen
  (params (Position :type Vector) (Padding :type Float%20%28single-precision%29))
  (bind _returnvalue (Viewport|GetViewportSize))
  (bind _returnvalue_2 (Viewport|GetViewportSize))
  (bind _returnvalue_3 (Game|GetPlayerController 0))
  (bind (_screenposition _returnvalue_4) (Class|GameplayStatics|ProjectWorldtoScreen _returnvalue_3 Position false))
  (bind (_x _y) (Math|Vector2D|BreakVector2D _returnvalue))
  (bind (_x_2 _y_2) (Math|Vector2D|BreakVector2D _returnvalue_2))
  (bind (_x_3 _y_3) (Math|Vector2D|BreakVector2D _screenposition))
  (LocalVariables|SetPaddingX (* Padding _x_2))
  (LocalVariables|SetPaddingY (* Padding _y_2))
  (if _returnvalue_4
    (return (Math|Boolean|ANDBoolean (>= _x_3 (LocalVariables|GetPaddingX)) (>= _y_3 (LocalVariables|GetPaddingX)) (<= (+ _x_3 (LocalVariables|GetPaddingX)) _x) (<= (+ _y_3 (LocalVariables|GetPaddingX)) _y)))
    (else
      (return false))))

(fn CalculateLocation
  (return (Math|Transform|MakeTransform (+ (Variables|Default|GetCurrentAimPoint) (* (Math|Vector|Normalize (Math|Vector|NegateVector (Variables|Default|GetDirection))) (Variables|Default|GetDistance))) (Variables|Default|GetCameraRotation))))

(fn CalculateClippingDistance
  (LocalVariables|SetSmallestDistance 1e+06)
  (for _array_element (Variables|Default|GetActors)
    (LocalVariables|SetSmallestDistance (Math|Float|Min(Float) (Math|Vector|VectorLength (- (Transformation|GetActorLocation) (Transformation|GetActorLocation _array_element))) (LocalVariables|GetSmallestDistance))))
  (return (Math|Float|Min(Float) (* (LocalVariables|GetSmallestDistance) 0.5) (Utilities|GetMaxNear))))

(fn GetAimPoint
  (return (Utilities|SetHeight (Math|Vector|GetVectorArrayAverage (Variables|Default|GetTargets)) 1e+02)))

(fn UpdateLocation
  (params (SetNativeCamera :type Boolean))
  (bind _maincamera (Variables|Default|GetMainCamera))
  (bind _yawpitch (Variables|Default|GetYawPitch))
  (bind (_x _y) (Math|Vector2D|BreakVector2D _yawpitch))
  (bind _transform (CallFunction|CalculateLocation))
  (Transformation|SetActorTransform _transform)
  (if SetNativeCamera
    (Default|SetExternalYawOverride _maincamera true _x)
    (Default|SetExternalPitchOverride _maincamera true _y)
    (Class|BtlCamera|SetFocusLocation _maincamera (Variables|Default|GetCurrentAimPoint))))

(fn OnInitialActivate
  (Variables|Default|SetCurrentAimPoint "0, 0, 0")
  (Variables|Default|SetYawPitch "")
  (Variables|Default|SetDistance 1.5e+03))

(fn OnDeactivate
  (bind _maincamera (Variables|Default|GetMainCamera))
  (bind _yawpitch (Variables|Default|GetYawPitch))
  (bind (_x _y) (Math|Vector2D|BreakVector2D _yawpitch))
  (if (Variables|Default|GetIsActive)
    (Variables|Default|SetIsActive false)
    (Default|NativeResetNearClippingPlane (Variables|Default|GetMod))
    (Actor|Tick|SetActorTickEnabled false)
    (Utilities|IsValid _maincamera
      (:Is%20Valid
        (Default|SetExternalYawOverride _maincamera false _x)
        (Default|SetExternalPitchOverride _maincamera false _y)))))

(fn OnActivate
  (Variables|Default|SetIsActive true)
  (Actor|Tick|SetActorTickEnabled true)
  (Class|ActorComponent|SetTickablewhenPaused (Variables|CameraActor|GetCameraComponent) true))