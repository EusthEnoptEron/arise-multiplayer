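; BP_ModHelper is a utility Blueprint for the multiplayer mod, covering screen checks, player colors, UI visibility and controller access.
; IsOnScreen tests a projected world position against viewport-relative padding, while small helpers map booleans to visibility and player indices to colors.
; Native_ functions are stubs for HUD, widget and controller calls, returning defaults or just printing.
; GetControllers presizes an array from the native count and passes it to Native_GetControllers to fill.
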(fn IsonScreen
  (params (Position :type Vector) (Padding :type Float%20%28single-precision%29))
  (bind _returnvalue (Viewport|GetViewportSize))
  (bind _returnvalue_2 (Viewport|GetViewportSize))
  (bind _returnvalue_3 (Game|GetPlayerController 0))
  (bind (_screenposition _returnvalue_4) (Class|GameplayStatics|ProjectWorldtoScreen _returnvalue_3 Position false))
  (bind (_x _y) (Math|Vector2D|BreakVector2D _returnvalue))
  (bind (_x_2 _y_2) (Math|Vector2D|BreakVector2D _returnvalue_2))
  (bind (_x_3 _y_3) (Math|Vector2D|BreakVector2D _screenposition))
  (LocalVariables|SetPaddingX (* Padding _x_2))
  (LocalVariables|SetPaddingY (* Padding _y_2))
  (if _returnvalue_4
    (return (Math|Boolean|ANDBoolean (>= _x_3 (LocalVariables|GetPaddingX)) (>= _y_3 (LocalVariables|GetPaddingY)) (<= (+ _x_3 (LocalVariables|GetPaddingX)) _x) (<= (+ _y_3 (LocalVariables|GetPaddingY)) _y)))
    (else
      (return false))))

(fn NativeGetHudVisibility
  (params (Name :type String))
  (return "Visible"))

(fn NativeGetRootWidget
  (params (UserWidget :type User%20Widget%20Object%20Reference))
  (return 0))

(fn BooltoVisibility
  (params (IsVisible :type Boolean))
  (if IsVisible
    (return "Visible")
    (else
      (return "Collapsed"))))

(fn NativePrintWidgetHierarchy
  (params (Widget :type User%20Widget%20Object%20Reference)))

(fn GetPlayerColor
  (params (Index :type Integer))
  (switch int Index
    (:Default
      _)
    (:0
      _)
    (:1
      (return (Math|Color|MakeColor 0 0 150 255)))
    (:2
      (return (Math|Color|MakeColor 0 100 0 255)))
    (:3
      (return (Math|Color|MakeColor 100 0 100 255))))
  (return (Math|Color|MakeColor 150 0 0 255)))

(fn NativeGetControllers
  (params (NewParam :type Array%20of%20Controller%20Data%20Object%20References))
  (return))

(fn NativeSetControllers
  (params (Controllers :type Array%20of%20Controller%20Data%20Object%20References)))

(fn NativeSetVibration
  (params (Id :type String) (IsOn :type Boolean))
  (Development|PrintString 0 (Utilities|String|Append "Vibration: " (Utilities|String|ToString(Boolean) IsOn) Id)))

(fn NativeGetControllerCount
  (return 0))

(fn GetControllers
  (bind _result (LocalVariables|GetResult))
  (bind _count (CallFunction|NativeGetControllerCount))
  (Utilities|Array|Resize _result _count)
  (CallFunction|NativeGetControllers _result)
  (return (LocalVariables|GetResult)))